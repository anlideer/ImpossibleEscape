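; Destructible wall built with Geometry Script that gets holes carved into it at hit points.
; On rebuild it generates a box from MeshSize and enables complex-as-simple collision.
; BeginPlay caches a sphere mesh of ProjectileRadius as the cutting tool.
; The Destruction event converts the impact point to local space and boolean-subtracts that sphere from the wall mesh at runtime.
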(event EventDestruction
  (params (Hit :type Hit%20Result%20Structure))
  (Utilities|IsValid (Variables|Default|GetProjectileMesh)
    (:Is%20Valid
      (GeometryScript|Booleans|ApplyMeshBoolean :TargetMesh (Variables|Default|GetTarget%20Mesh) :ToolMesh (Variables|Default|GetProjectileMesh) :ToolTransform (Math|Transform|MakeTransform (Math|Transform|InverseTransformLocation (Transformation|GetWorldTransform (Variables|DynamicMeshActor|GetDynamicMeshComponent)) (.ImpactPoint (Collision|BreakHitResult Hit))) "0, 0, 0" "1.000000,1.000000,1.000000") :Operation "Subtract" :Debug 0))))

(event Events|EventOnRebuildGeneratedMesh
  (params (TargetMesh :type Dynamic%20Mesh%20Object%20Reference))
  (bind _meshsize (Variables|Default|GetMeshSize))
  (bind _output_get (Variables|Default|SetTarget%20Mesh TargetMesh))
  (Class|GeometryScriptLibraryMeshPrimitiveFunctions|AppendBox :TargetMesh _output_get :DimensionX (.x _meshsize) :DimensionY (.y _meshsize) :DimensionZ (.z _meshsize) :Debug 0)
  (Class|DynamicMeshComponent|EnableComplexasSimpleCollision (Variables|DynamicMeshActor|GetDynamicMeshComponent)))

(event EventBeginPlay
  (bind _returnvalue (DynamicMeshActor|AllocateComputeMesh))
  (bind _returnvalue_2 (Class|GeometryScriptLibraryMeshPrimitiveFunctions|AppendSphereBox :TargetMesh _returnvalue :Radius (Variables|Default|GetProjectileRadius) :Debug 0))
  (Variables|Default|SetProjectileMesh _returnvalue_2))

(fn ConstructionScript)